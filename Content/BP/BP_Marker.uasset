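; BP_Marker is a world marker actor that shows a colored icon and the player's distance to it, and registers itself on the compass.
; Construction tints the cone material with MarkerColor.
; BeginPlay sets the MarkerWidget's color and icon, and after a short delay creates a WDG_CompassMarker in the viewport, initialized with this actor as owner.
; Tick updates the widget text with the truncated distance in meters.
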(event `self.ReceiveBeginPlay`
  (bind _marker (`self.marker`))
  (`KismetSystemLibrary.Delay` 0.2)
  (bind _returnvalue (`|CreateWidget` "/Game/UI/WDG_CompassMarker.WDG_CompassMarker_C"))
  (set `self.marker` _returnvalue)
  (`UserWidget.AddToViewport` _marker 0)
  (`/Game/UI/WDG_CompassMarker.InitializeMarker` _marker (`self.Marker Material`) (`self.Marker Color`) self)
  (message `/Game/UI/BPI_MarkerWidget.setMarkerColor` (`WidgetComponent.GetUserWidgetObject` (`self.markerWidget`)) (`self.Marker Color`))
  (message `/Game/UI/BPI_MarkerWidget.setMarkerIcon` (`WidgetComponent.GetUserWidgetObject` (`self.markerWidget`)) (`self.markerIcon`)))

(event `self.ReceiveTick`
  (params (DeltaSeconds :type "Float (single-precision)"))
  (message `/Game/UI/BPI_MarkerWidget.updateText` (`WidgetComponent.GetUserWidgetObject` (`self.markerWidget`)) (`KismetTextLibrary.Conv_StringToText` (`KismetStringLibrary.Concat_StrStr` (`KismetStringLibrary.Conv_IntToString` (`KismetMathLibrary.FTrunc` (/ (`KismetMathLibrary.Vector_Distance` (`self.K2_GetActorLocation` (`GameplayStatics.GetPlayerCharacter` 0)) (`self.K2_GetActorLocation`)) 100.0))) " m"))))

(fn `UserConstructionScript`
  (`MeshComponent.SetVectorParameterValueOnMaterials` (`self.Cone`) "Color" (`KismetMathLibrary.Conv_LinearColorToVector` (`self.Marker Color`))))